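; BP_AudioPlayer is an actor that prepares a streaming sound wave for runtime audio on its Audio component.
; On BeginPlay it waits a tick, creates the streaming sound wave, stores it and assigns it to the component.
; After another tick it pre-allocates a small audio data buffer and prints whether that succeeded.
; The graph never appends audio data or explicitly starts playback.
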(event `self.ReceiveBeginPlay`
  (`KismetSystemLibrary.DelayUntilNextTick`)
  (bind _returnvalue (`StreamingSoundWave.CreateStreamingSoundWave`))
  (bind _output_get (set `self.MySoundWave` _returnvalue))
  (`AudioComponent.SetSound` (`self.Audio`) _output_get)
  (`KismetSystemLibrary.DelayUntilNextTick`)
  (`StreamingSoundWave.PreAllocateAudioData` (`self.MySoundWave`) 5000 (delegate `CustomEvent`)))

(event `CustomEvent`
  (params (bSucceeded :type Boolean))
  (`KismetSystemLibrary.PrintString` (`KismetStringLibrary.Conv_BoolToString` bSucceeded)))

(fn `UserConstructionScript`)