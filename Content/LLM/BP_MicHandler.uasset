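; BP_MicHandler is a push-to-talk microphone test that records while C is held, then plays the recording back.
; It uses Runtime Audio Importer, lists input devices at BeginPlay and appends captured float samples to a byte buffer that is never cleared.
; After release and a short delay, the buffer is imported as raw stereo audio, played, and exported to Ogg Opus, with only the byte count printed.
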(event `OnPopulateAudioData_Event`
  (params (PopulatedAudioData :type "Array of Float (single-precision) (by ref)"))
  (`KismetArrayLibrary.Array_Append` (`self.Buffer`) (`RuntimeAudioUtilities.ConvertFloatArrayToBytes` PopulatedAudioData)))

(event `GetAvailableAudioInputDevices_Event`
  (params (AvailableDevices :type "Array of RuntimeAudioInputDeviceInfo Structure (by ref)"))
  (for (_array_element _array_index) AvailableDevices
    (`KismetSystemLibrary.PrintString` (`KismetTextLibrary.Conv_TextToString` (`|FormatText` "Idx: {Idx}, Name: {Name}" _array_index (break `RuntimeAudioInputDeviceInfo` _array_element))))))

(event `self.ReceiveBeginPlay`
  (`|ExecutionSequence`
    (:`then_0`
      (bind _returnvalue (`CapturableSoundWave.CreateCapturableSoundWave`))
      (bind _output_get (set `self.CapturableSoundWave` _returnvalue))
      (add `ImportedSoundWave.OnPopulateAudioData` _output_get (delegate `OnPopulateAudioData_Event`))
      (`CapturableSoundWave.GetAvailableAudioInputDevices` (delegate `GetAvailableAudioInputDevices_Event`)))
    (:`then_1`
      (bind _returnvalue_2 (`RuntimeAudioImporterLibrary.CreateRuntimeAudioImporter`))
      (bind _output_get_2 (set `self.RuntimeAudioImporter` _returnvalue_2))
      (add `RuntimeAudioImporterLibrary.OnResult` _output_get_2 (delegate `OnResult_Event`)))))

(event `OnResult_Event`
  (params (Importer :type "RuntimeAudioImporterLibrary Object Reference") (ImportedSoundWave :type "ImportedSoundWave Object Reference") (Status :type "ERuntimeImportStatus Enum" :default "SuccessfulImport"))
  (`GameplayStatics.PlaySound2D` ImportedSoundWave 1.0 1.0 0.0 null null)
  (`RuntimeAudioExporter.ExportSoundWaveToBuffer` ImportedSoundWave "OggOpus" 0 (make `RuntimeAudioExportOverrideOptions` 2 48000) (delegate `ExportSoundWaveToBuffer_Event`)))

(event `ExportSoundWaveToBuffer_Event`
  (params (bSucceeded :type Boolean) (AudioData :type "Array of Byte (by ref)"))
  (if bSucceeded
    (`KismetSystemLibrary.PrintString` (`KismetStringLibrary.Conv_IntToString` (`KismetArrayLibrary.Array_Length` AudioData)))))

(event `Key|C`
  (params (Key :type "Key Structure"))
  (bind _capturablesoundwave (`self.CapturableSoundWave`))
  (:`Pressed`
    (`CapturableSoundWave.StartCapture` _capturablesoundwave 0))
  (:`Released`
    (`CapturableSoundWave.StopCapture` _capturablesoundwave)
    (`KismetSystemLibrary.Delay` 2.0)
    (`RuntimeAudioImporterLibrary.ImportAudioFromRAWBuffer` (`self.RuntimeAudioImporter`) (`self.Buffer`) "Float32" 48000 2)))

(fn `UserConstructionScript`)